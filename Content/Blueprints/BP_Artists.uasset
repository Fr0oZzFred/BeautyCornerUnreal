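; BP_Artists loads artist data and hands it to the artists panel of the scene UI.
; One tick after BeginPlay, it looks up each ArtistsArray name in DT_Artists, storing rows at matching indices in Artists and printing any missing names.
; It then finds the first top-level W_Scene widget, copies the array into its WArtists child and calls Init on that child.
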(event `self.ReceiveBeginPlay`
  (`KismetSystemLibrary.DelayUntilNextTick`)
  (`|ExecutionSequence`
    (:`then_0`
      (for (_array_element _array_index) (`self.ArtistsArray`)
        (bind _returnvalue (`|GetDataTableRow` "/Game/HAE_BlenderProjects/DT_Artists.DT_Artists" _array_element)
          (:`then`
            (`KismetArrayLibrary.Array_Set` (`self.Artists`) _array_index _returnvalue))
          (:`RowNotFound`
            (`KismetSystemLibrary.PrintString` (`KismetStringLibrary.Concat_StrStr` (`KismetStringLibrary.Conv_NameToString` _array_element) " Not Found"))))))
    (:`then_1`
      (bind _foundwidgets (`WidgetBlueprintLibrary.GetAllWidgetsOfClass` "/Game/Widgets/W_Scene.W_Scene_C"))
      (bind _w_artists (`/Game/Widgets/W_Scene.W_Artists` (`|GetArrayItem` _foundwidgets)))
      (set `/Game/Widgets/W_Artists.Artists` (`self.Artists`) _w_artists)
      (`/Game/Widgets/W_Artists.Init` _w_artists))))

(fn `UserConstructionScript`)